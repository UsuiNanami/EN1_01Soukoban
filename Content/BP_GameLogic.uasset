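; BP_GameLogic runs a one-dimensional, Sokoban-style push game on an array of enum cells.
; BeginPlay adds the input mapping context, then horizontal input finds the player cell and moves it by the truncated axis value.
; MoveObject recursively pushes chains of one blocking type, failing at array bounds and overwriting any other target cell.
; The field is printed as a keyed debug string at start and after each input.
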(event Input|EnhancedActionEvents|EnhancedInputActionIA_Horizontal
  (params (ActionValue :type Float%20%28double-precision%29) (ElapsedSeconds :type Float%20%28double-precision%29) (TriggeredSeconds :type Float%20%28double-precision%29) (InputAction :type Input%20Action%20Object%20Reference :default "/Game/IA_Horizontal.IA_Horizontal"))
  (bind _playerindex (CallFunction|GetPlayerIndex))
  (デフォルト|MoveObject _playerindex (Math|Float|Truncate ActionValue))
  (CallFunction|PrintFieldObjects))

(event EventBeginPlay
  (Input|AddMappingContext (PlayerController|LocalPlayerSubsystems|GetEnhancedInputLocalPlayerSubsystem (Game|GetPlayerController 0)) "/Game/IMC_InGame.IMC_InGame" 0 "(bIgnoreAllPressedKeysUntilRelease=True,bForceImmediately=False,bNotifyUserSettings=False)")
  (CallFunction|PrintFieldObjects))

(event Collision|EventActorBeginOverlap
  (params (OtherActor :type Actor%20Object%20Reference)))

(event EventTick
  (params (DeltaSeconds :type Float%20%28single-precision%29)))

(event Input|KeyboardEvents|DebugKeyA
  (params (Key :type Key%20Structure) (ActionValue :type Input%20Action%20Value%20Structure)))

(fn ConstructionScript)

(fn PrintFieldObjects
  (Variables|Default|SetDebugStringBuffer "")
  (for _array_element (Variables|Default|GetFieldObiects)
    (Variables|Default|SetDebugStringBuffer (Utilities|String|Append (Variables|Default|GetDebugStringBuffer) "" (Utilities|String|ToString(Integer) (Math|Conversions|ToInteger(Byte) _array_element)))))
  (Development|PrintString (Variables|Default|GetDebugStringBuffer) true true "(R=0.000000,G=0.660000,B=1.000000,A=1.000000)" 3e+02 "PrintFieldObjects"))

(fn GetPlayerIndex
  (for (_array_element _array_index) (Variables|Default|GetFieldObiects)
    (if (Utilities|Enum|Equal(Enum) _array_element "NewEnumerator1")
      (return _array_index)))
  (return -1))

(fn MoveObject
  (params (MoveFromIndex :type Integer) (Velocity :type Integer))
  (bind _output_get (LocalVariables|SetMoveToIndex (+ MoveFromIndex Velocity 0)))
  (if (Utilities|Array|IsValidIndex (Variables|Default|GetFieldObiects) _output_get)
    (if (Utilities|Enum|NotEqual(Enum) (Utilities|Array|Get(acopy) (Variables|Default|GetFieldObiects) (LocalVariables|GetMoveToIndex)) "NewEnumerator4")
      _
      (else
        (bind _suceeded (デフォルト|MoveObject (LocalVariables|GetMoveToIndex) Velocity))
        (if _suceeded
          _
          (else
            (return false)))))
    (Utilities|Array|SetArrayElem (Variables|Default|GetFieldObiects) (LocalVariables|GetMoveToIndex) (Utilities|Array|Get(acopy) (Variables|Default|GetFieldObiects) MoveFromIndex))
    (Utilities|Array|SetArrayElem (Variables|Default|GetFieldObiects) MoveFromIndex "NewEnumerator0")
    (return true)
    (else
      (return false))))